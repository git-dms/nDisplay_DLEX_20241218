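; Door actor Blueprint that swings a pair of doors open when its OpenDoor event is called.
; OpenDoor plays a timeline whose float track drives the yaw of the DoorOriginR pivot and, negated, the DoorOriginL pivot, so the two sides rotate in mirror image.
; The file has no close logic or trigger of its own, as its overlap, BeginPlay and Tick events are disabled.
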(event `self.OpenDoor`
  (bind (_direction _animation) (`Timeline|Timeline_0`)
    (:`Update`
      (`|ExecutionSequence`
        (:`then_0`
          (`SceneComponent.K2_SetRelativeRotation` (`self.DoorOriginR`) (`KismetMathLibrary.MakeRotator` 0.0 0.0 _animation) false false))
        (:`then_1`
          (`SceneComponent.K2_SetRelativeRotation` (`self.DoorOriginL`) (`KismetMathLibrary.MakeRotator` 0.0 0.0 (* _animation -1.0)) false false))))))

(fn `UserConstructionScript`
  (`parent.UserConstructionScript`))